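; Enemy actor with a simple health pool that can be damaged and killed.
; Health starts at MaxHealth on BeginPlay.
; TakeDamage spawns a HurtFX actor at the enemy's transform, scaled up but flat on Y, then either subtracts the damage or calls Die when health would reach zero.
; Die prints a message and destroys the actor.
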(event Custom|Die
  (Development|PrintString "I died")
  (Actor|DestroyActor))

(event EventBeginPlay
  (Variables|Default|SetHealth (Variables|Default|GetMaxHealth)))

(event Collision|EventActorBeginOverlap
  (params (OtherActor :type Actor%20Object%20Reference)))

(event EventTick
  (params (DeltaSeconds :type Float%20%28single-precision%29)))

(fn ConstructionScript)

(fn TakeDamage
  (params (Damage :type Float%20%28double-precision%29))
  (bind _returnvalue (Game|SpawnActorfromClass "/Game/Effects/HurtFX.HurtFX_C" (Transformation|GetActorTransform) "AlwaysSpawn" 0 0))
  (Transformation|SetActorScale3D _returnvalue "2.000000, 0,2.000000")
  (if (<= (- (Variables|Default|GetHealth) Damage) 0.0)
    (CallFunction|Die)
    (else
      (Variables|Default|SetHealth (- (Variables|Default|GetHealth) Damage)))))