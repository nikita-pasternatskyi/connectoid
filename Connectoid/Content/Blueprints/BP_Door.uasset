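; BP_Door is a level exit for a 2D game that lets the player travel to the level set in NextLevel.
; A text prompt stays hidden until BP_Player2D overlaps the Box trigger, which also enables the door's input, and both switch off when the player leaves.
; Pressing the Trigger action while input is enabled calls LoadLevel on BP_2DGameMode.
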(event OnComponentBeginOverlap(Box)
  (params (OverlappedComponent :type Primitive%20Component%20Object%20Reference) (OtherActor :type Actor%20Object%20Reference) (OtherComp :type Primitive%20Component%20Object%20Reference) (OtherBodyIndex :type Integer) (bFromSweep :type Boolean) (SweepResult :type Hit%20Result%20Structure%20%28by%20ref%29))
  ;[1 1 1] Show text
  (Utilities|Casting|CastToBP_Player2D OtherActor)
  (Rendering|SetVisibility (Variables|Default|GetTextRender) true false)
  (Input|EnableInput (Game|GetPlayerController 0)))

(event OnComponentEndOverlap(Box)
  (params (OverlappedComponent :type Primitive%20Component%20Object%20Reference) (OtherActor :type Actor%20Object%20Reference) (OtherComp :type Primitive%20Component%20Object%20Reference) (OtherBodyIndex :type Integer))
  ;[1 1 1] Hide text
  (Utilities|Casting|CastToBP_Player2D OtherActor)
  (Rendering|SetVisibility (Variables|Default|GetTextRender) false false)
  (Input|DisableInput (Game|GetPlayerController 0)))

(event EventBeginPlay
  ;[1 1 1] Turn off text
  (Rendering|SetVisibility (Variables|Default|GetTextRender) false false))

(event Input|ActionEvents|InputActionTrigger
  (params (Key :type Key%20Structure :default "None"))
  ;[1 1 1] Load level when Trigger
  (:Pressed
    (bind _asbp_2dgame_mode (Utilities|Casting|CastToBP_2DGameMode (Game|GetGameMode)))
    (Default|LoadLevel _asbp_2dgame_mode (Variables|Default|GetNextLevel))))

(fn ConstructionScript)